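; BP_TennisBall is a physics-driven tennis ball that launches itself three seconds after play begins.
; Its Hit event branches on racket pawn, court or wall, playing a sound and applying a fixed impulse to return, bounce or rebound the ball.
; Racket hits have a one-second cooldown and reset velocity first beyond an X threshold.
; Wall bounce sounds play at the world origin, not at the ball.
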(event `self.ReceiveBeginPlay`
  (`KismetSystemLibrary.Delay` 3.0)
  (`PrimitiveComponent.SetEnableGravity` (`self.Sphere`) true)
  (`PrimitiveComponent.AddImpulse` (`self.StaticMesh`) (1500.0 400.0 0.0) "None" true))

(event `self.ReceiveHit`
  (params (MyComp :type "PrimitiveComponent Object Reference") (Other :type "Actor Object Reference") (OtherComp :type "PrimitiveComponent Object Reference") (bSelfMoved :type Boolean) (HitLocation :type "Vector Structure") (HitNormal :type "Vector Structure") (NormalImpulse :type "Vector Structure") (Hit :type "HitResult Structure (by ref)"))
  (bind _returnvalue (`SceneComponent.K2_GetComponentLocation` (`self.Sphere`)))
  (cast `/Game/Blueprints/BP_Racket2Pawn` Other
    (:`then`
      (if (`self.HitReady`)
        (`GameplayStatics.PlaySoundAtLocation` "/Game/Sounds/TennisHitSound.TennisHitSound" _returnvalue (struct) 1.0 1.0 0.0 null null null null)
        (if (> (.x _returnvalue) 1136.060281)
          (`PrimitiveComponent.SetAllPhysicsLinearVelocity` (`self.Sphere`) (`self.stopBall`) false)
          (`PrimitiveComponent.AddImpulse` (`self.Sphere`) (-2500.0 0.0 600.0) "None" false)
          (else
            (`PrimitiveComponent.AddImpulse` (`self.Sphere`) (-2500.0 0.0 600.0) "None" false)))
        (set `self.HitReady` false)
        (`KismetSystemLibrary.Delay` 1.0)
        (set `self.HitReady` true)))
    (:`CastFailed`
      (cast `/Game/Blueprints/Court` Other
        (:`then`
          (`GameplayStatics.PlaySoundAtLocation` "/Game/Sounds/TennisBounceSound.TennisBounceSound" _returnvalue (struct) 1.0 1.0 0.0 null null null null)
          (`PrimitiveComponent.AddImpulse` (`self.Sphere`) (0.0 0.0 100.0) "None" false))
        (:`CastFailed`
          (cast `/Game/Blueprints/Wall` Other)
          (`GameplayStatics.PlaySoundAtLocation` "/Game/Sounds/TennisBounceSound.TennisBounceSound" (0.0 0.0 0.0) (struct) 1.0 1.0 0.0 null null null null)
          (`PrimitiveComponent.AddImpulse` (`self.Sphere`) (1500.0 0.0 400.0) "None" false))))))

(fn `UserConstructionScript`)